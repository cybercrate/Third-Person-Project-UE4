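; Game instance that owns the game's menu flow: loading screen, main, settings and pause menus, plus a confirm prompt for quitting to the main menu.
; Each event lazily creates and caches its widget, then adds or removes it while switching input mode, cursor visibility and pause state.
; New game shows the loading screen and waits a fixed delay before opening the World level.
; A one-shot macro centers the mouse when the main menu appears.
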(event Custom|Show%20Main%20Menu
  (bind _returnvalue (Game|GetPlayerController 0))
  ;[1 1 1] Call MainMenu and show mouse cursor
  (Utilities|IsValid (Variables|Widgets|GetMain%20Menu%20WB)
    (:Is%20Valid
      _)
    (:Is%20Not%20Valid
      (bind _returnvalue_2 (UserInterface|CreateWidget "/Game/UI/Menus/MainMenu_WB.MainMenu_WB_C" _returnvalue))
      (Variables|Widgets|SetMain%20Menu%20WB _returnvalue_2)))
  (UserInterface|Viewport|AddtoViewport (Variables|Widgets|GetMain%20Menu%20WB) 0)
  (Variables|/Script/Engine.PlayerController|SetbShowMouseCursor _returnvalue true)
  (Input|SetInputModeUIOnly _returnvalue (Variables|Widgets|GetMain%20Menu%20WB) "LockInFullscreen")
  (Utilities|CursortoCenter))

(event Custom|Show%20Settings%20Menu
  ;[1 1 1] Call SettingsMenu
  (Utilities|IsValid (Variables|Widgets|GetSettings%20Menu%20WB)
    (:Is%20Valid
      _)
    (:Is%20Not%20Valid
      (bind _returnvalue (UserInterface|CreateWidget "/Game/UI/Menus/SettingsMenu_WB.SettingsMenu_WB_C" (Game|GetPlayerController 0)))
      (Variables|Widgets|SetSettings%20Menu%20WB _returnvalue)))
  (UserInterface|Viewport|AddtoViewport (Variables|Widgets|GetSettings%20Menu%20WB) 0))

(event Custom|PauseMenu%20To%20MainMenu%20Calcel
  ;[1 1 1] From PauseMenu to MainMenu
  (Widget|RemovefromParent (Variables|Widgets|GetPause%20Menu%20To%20Main%20Menu%20WB))
  (UserInterface|Viewport|AddtoViewport (Variables|Widgets|GetPause%20Menu%20WB) 0))

(event Custom|Create%20New%20Game
  (bind _returnvalue (Game|GetPlayerController 0))
  ;[1 1 1] Start new game
  (Variables|/Script/Engine.PlayerController|SetbShowMouseCursor _returnvalue false)
  (Input|SetInputModeGameOnly _returnvalue)
  (CallFunction|ShowLoadingScreen)
  (Utilities|FlowControl|Delay 4.0)
  (Game|OpenLevel(byName) "World"))

(event Custom|Show%20Loading%20Screen
  ;[1 1 1] Show loading screen
  (Utilities|IsValid (Variables|Widgets|GetLoading%20Screen%20WB)
    (:Is%20Valid
      _)
    (:Is%20Not%20Valid
      (bind _returnvalue (UserInterface|CreateWidget "/Game/UI/Menus/LoadingScreen_WB.LoadingScreen_WB_C" (Game|GetPlayerController 0)))
      (Variables|Widgets|SetLoading%20Screen%20WB _returnvalue)))
  (UserInterface|Viewport|AddtoViewport (Variables|Widgets|GetLoading%20Screen%20WB) 0))

(event Custom|Show%20Pause%20Menu
  (bind _returnvalue (Game|GetPlayerController 0))
  ;[1 1 1] Call PauseMenu
  (Utilities|IsValid (Variables|Widgets|GetPause%20Menu%20WB)
    (:Is%20Valid
      _)
    (:Is%20Not%20Valid
      (bind _returnvalue_2 (UserInterface|CreateWidget "/Game/UI/Menus/PauseMenu_WB.PauseMenu_WB_C" _returnvalue))
      (Variables|Widgets|SetPause%20Menu%20WB _returnvalue_2)))
  (UserInterface|Viewport|AddtoViewport (Variables|Widgets|GetPause%20Menu%20WB) 0)
  (Input|SetInputModeUIOnly _returnvalue (Variables|Widgets|GetPause%20Menu%20WB) "LockInFullscreen")
  (Game|SetGamePaused true)
  (Variables|/Script/Engine.PlayerController|SetbShowMouseCursor _returnvalue true))

(event Custom|Pause%20Menu%20Resume
  (bind _returnvalue (Game|GetPlayerController 0))
  ;[1 1 1] From PauseMenu back to Game
  (Widget|RemovefromParent (Variables|Widgets|GetPause%20Menu%20WB))
  (Game|SetGamePaused false)
  (Input|SetInputModeGameOnly _returnvalue)
  (Variables|/Script/Engine.PlayerController|SetbShowMouseCursor _returnvalue false))

(event Custom|From%20PauseMenu%20To%20MainMenu
  ;[1 1 1] From PauseMenu to MainMenu
  (Utilities|IsValid (Variables|Widgets|GetPause%20Menu%20To%20Main%20Menu%20WB)
    (:Is%20Valid
      _)
    (:Is%20Not%20Valid
      (bind _returnvalue (UserInterface|CreateWidget "/Game/UI/Menus/PauseToMainMenu_WB.PauseToMainMenu_WB_C" (Game|GetPlayerController 0)))
      (Variables|Widgets|SetPause%20Menu%20To%20Main%20Menu%20WB _returnvalue)))
  (UserInterface|Viewport|AddtoViewport (Variables|Widgets|GetPause%20Menu%20To%20Main%20Menu%20WB) 0)
  (Widget|RemovefromParent (Variables|Widgets|GetPause%20Menu%20WB)))

(event Custom|Pause%20Menu:%20Show%20Settings%20Menu
  ;[1 1 1] Call SettingsMenu from PauseMenu
  (Widget|RemovefromParent (Variables|Widgets|GetPause%20Menu%20WB))
  (Utilities|IsValid (Variables|Widgets|GetPause%20Settings%20Menu%20WB)
    (:Is%20Valid
      _)
    (:Is%20Not%20Valid
      (bind _returnvalue (UserInterface|CreateWidget "/Game/UI/Menus/PauseSettingsMenu_WB.PauseSettingsMenu_WB_C"))
      (Variables|Widgets|SetPause%20Settings%20Menu%20WB _returnvalue)))
  (UserInterface|Viewport|AddtoViewport (Variables|Widgets|GetPause%20Settings%20Menu%20WB) 0))

(event Custom|PauseMenu%20To%20MainMenu%20Confirm
  ;[1 1 1] From PauseMenu to MainMenu
  (Game|OpenLevel(byName) "MainMenu"))

(event Custom|Pause%20Settings%20Menu%20To%20Pause%20Menu
  ;[1 1 1] Back from Pause Settings Menu to Pause Menu
  (Widget|RemovefromParent (Variables|Widgets|GetPause%20Settings%20Menu%20WB))
  (UserInterface|Viewport|AddtoViewport (Variables|Widgets|GetPause%20Menu%20WB) 0))